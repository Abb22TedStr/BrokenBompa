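; Game mode for the horror game's menu and lobby that tracks connected player controllers and shares their profiles.
; New players pass through a level-name switch, then are added to the player list and told to create the lobby menu and run initial setup.
; Logout removes the controller and calls UpdateLobby, which rebuilds the profile list and pushes it to every remaining controller to update displayed names.
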(event Custom|UpdateLobby
  (params (PlayerNames :type Boolean))
  (if PlayerNames
    (Utilities|Array|Clear (Variables|Default|GetAll_PlayerProfiles))
    (for _array_element (Variables|Default|GetAll_ConnectedPlayers)
      (Utilities|Array|Add (Variables|Default|GetAll_PlayerProfiles) (Variables|/Game/Framework/BP_HorrorMenu_Controller.BP_HorrorMenu_Controller_C|GetPlayer%20Profile _array_element)))
    (for _array_element_2 (Variables|Default|GetAll_ConnectedPlayers)
      (if PlayerNames
        (Default|UpdatePlayerNames _array_element_2 (Variables|Default|GetAll_PlayerProfiles))))))

(event EventBeginPlay)

(event EventTick
  (params (DeltaSeconds :type Float%20%28single-precision%29)))

(event EventHandleStartingNewPlayer
  (params (NewPlayer :type Player%20Controller%20Object%20Reference))
  (bind _returnvalue (Game|GetCurrentLevelName true))
  (switch string _returnvalue
    (:LobbyMenu_Map
      (bind _asbp_horror_menu_controller (Utilities|Casting|CastToBP_HorrorMenu_Controller NewPlayer))
      (Utilities|Array|Add (Variables|Default|GetAll_ConnectedPlayers) _asbp_horror_menu_controller)
      (Default|CreateLobbyMenu _asbp_horror_menu_controller)
      (Default|InitialSetup _asbp_horror_menu_controller))))

(event EventOnLogout
  (params (ExitingController :type Controller%20Object%20Reference))
  (bind _asbp_horror_menu_controller (Utilities|Casting|CastToBP_HorrorMenu_Controller ExitingController))
  (Utilities|Array|RemoveItem (Variables|Default|GetAll_ConnectedPlayers) _asbp_horror_menu_controller)
  (CallFunction|UpdateLobby true))

(fn ConstructionScript)