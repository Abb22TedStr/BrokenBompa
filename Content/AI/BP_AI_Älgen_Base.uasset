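; Base AI pawn for Älgen that, once possessed, finds a player character and chases it while alive.
; OnAISpawned polls FindEnemy every half second until it gets a target, then MoveToPlayer reissues AIMoveTo after each success or failure plus a delay.
; FindEnemy takes a lone player directly; with several it looks up the lowest attacker count, but its inverted index check (== -1) prevents valid selection.
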(event Custom|OnAISpawned
  (bind (_isvalidplayerfound _newenemy) (CallFunction|FindEnemy :!label _label))
  (if _isvalidplayerfound
    (Variables|Default|SetTargetPlayer _newenemy)
    (CallFunction|MovetoPlayer)
    (else
      (Utilities|FlowControl|Delay 0.5)
      (goto _label))))

(event Custom|MoveToPlayer
  (if (Variables|Default|GetIsAlive)
    (AI|AIMoveTo self "0, 0, 0" (Variables|Default|GetTargetPlayer) 1e+02 false
      (:OnSuccess
        _)
      (:OnFail
        _))
    (Utilities|FlowControl|Delay 2.0)
    (CallFunction|MovetoPlayer)))

(event EventPossessed
  (params (NewController :type Controller%20Object%20Reference))
  (bind _asbp_aicontroller_base (Utilities|Casting|CastToBP_AIController_Base NewController))
  (Variables|Default|SetAs%20BP%20AIController%20Base _asbp_aicontroller_base)
  (CallFunction|OnAISpawned))

(fn ConstructionScript)

(fn FindEnemy
  (bind _outactors (Actor|GetAllActorsOfClass "/Game/ThirdPerson/Blueprints/BP_ThirdPersonCharacter.BP_ThirdPersonCharacter_C"))
  (bind _output_get (LocalVariables|SetLcl_All_Players _outactors))
  (if (Utilities|Array|IsNotEmpty _output_get)
    (if (== (Utilities|Array|Length (LocalVariables|GetLcl_All_Players)) 1)
      (LocalVariables|SetLcl_IsValidPlayerFound true)
      (LocalVariables|SetLcl_NewEnemy (Utilities|Array|Get(acopy) (LocalVariables|GetLcl_All_Players)))
      (else
        (for _array_element (LocalVariables|GetLcl_All_Players)
          (Utilities|Array|Add (LocalVariables|GetLcl_AllAttackersNr) (Variables|/Game/ThirdPerson/Blueprints/BP_ThirdPersonCharacter.BP_ThirdPersonCharacter_C|GetNrAIAttackers _array_element)))
        (LocalVariables|SetLcl_LowestIndex (.IndexOfMinValue (Math|Integer|MinOfIntArray (LocalVariables|GetLcl_AllAttackersNr))))
        (if (== (LocalVariables|GetLcl_LowestIndex) -1)
          (Math|Integer|IncrementInt (Variables|/Game/ThirdPerson/Blueprints/BP_ThirdPersonCharacter.BP_ThirdPersonCharacter_C|GetNrAIAttackers (Utilities|Array|Get(acopy) (LocalVariables|GetLcl_All_Players) (LocalVariables|GetLcl_LowestIndex)))
            (:%20%20
              (LocalVariables|SetLcl_NewEnemy (Utilities|Array|Get(acopy) (LocalVariables|GetLcl_All_Players) (LocalVariables|GetLcl_LowestIndex)))
              (LocalVariables|SetLcl_IsValidPlayerFound true)))
          (else
            (LocalVariables|SetLcl_IsValidPlayerFound false)))))
    (else
      (LocalVariables|SetLcl_IsValidPlayerFound false)))
  (return (LocalVariables|GetLcl_IsValidPlayerFound) (LocalVariables|GetLcl_NewEnemy)))