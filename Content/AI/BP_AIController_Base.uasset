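; Base AI controller for Älgen AI pawns that makes them go after the player on sight.
; On possess it caches the pawn as BP_AI_Älgen_Base.
; AI Perception updates are filtered to successful sight of a BP_ThirdPersonCharacter that is not already TargetPlayer.
; The controller then passes that character to the pawn as its target and calls MoveToPlayer on it, with no handling for lost sight.
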(event OnTargetPerceptionUpdated(AIPerception)
  (params (Actor :type Actor%20Object%20Reference) (Stimulus :type AI%20Stimulus%20Structure))
  (bind _ai_älgen_base (Variables|Default|GetAI%20Älgen%20Base))
  (bind _returnvalue (Class|AIPerceptionSystem|GetSenseClassforStimulus Stimulus))
  (if (== _returnvalue "/Script/AIModule.AISense_Sight")
    (if (!= Actor (Variables|Default|GetTargetPlayer))
      (bind _asbp_third_person_character (Utilities|Casting|CastToBP_ThirdPersonCharacter Actor))
      (if (.bSuccessfullySensed (Utilities|Struct|BreakAIStimulus Stimulus))
        (Default|SetTargetPlayer _ai_älgen_base _asbp_third_person_character)
        (Default|MovetoPlayer _ai_älgen_base)))))

(event EventBeginPlay)

(event EventTick
  (params (DeltaSeconds :type Float%20%28single-precision%29)))

(event EventPossess
  (params (PossessedPawn :type Pawn%20Object%20Reference))
  (bind _asbp_ai_älgen_base (Utilities|Casting|CastToBP_AI_Älgen_Base PossessedPawn))
  (Variables|Default|SetAI%20Älgen%20Base _asbp_ai_älgen_base))

(fn ConstructionScript)